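; Pawn-style Blueprint that drives two physics pans, Panela1 and Panela2, with separate movement axes and reports their hits on Bolinha.
; Movement applies velocity-change impulses in X and Y.
; Jump fakes an arc on both pans with timed up and down impulse bursts, then cancels vertical motion using Panela1's Z velocity.
; Hits pass through DoOnce gates with delayed resets, set PanHited, and fire OnPanHit.
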(event OnComponentHit(Panela1)
  (params (HitComponent :type Primitive%20Component%20Object%20Reference) (OtherActor :type Actor%20Object%20Reference) (OtherComp :type Primitive%20Component%20Object%20Reference) (NormalImpulse :type Vector :default "0, 0, 0") (Hit :type Hit%20Result%20Structure%20%28by%20ref%29))
  (if (== OtherComp (Variables|Default|GetBolinha))
    (Utilities|FlowControl|DoOnce false :!label _label
      (:Completed
        (Utilities|FlowControl|Sequence
          (:then_0
            (Utilities|FlowControl|Delay 0.2)
            (goto _label Reset))
          (:then_1
            (bind _output_get (Variables|Default|SetPanHited 1))
            (Default|CallOnPanHit _output_get)))))))

(event OnComponentHit(Panela2)
  (params (HitComponent :type Primitive%20Component%20Object%20Reference) (OtherActor :type Actor%20Object%20Reference) (OtherComp :type Primitive%20Component%20Object%20Reference) (NormalImpulse :type Vector :default "0, 0, 0") (Hit :type Hit%20Result%20Structure%20%28by%20ref%29))
  (if (== OtherComp (Variables|Default|GetBolinha))
    (Utilities|FlowControl|DoOnce false :!label _label
      (:Completed
        (Utilities|FlowControl|Sequence
          (:then_0
            (Utilities|FlowControl|Delay 0.2)
            (goto _label Reset))
          (:then_1
            (bind _output_get (Variables|Default|SetPanHited 2))
            (Default|CallOnPanHit _output_get)))))))

(event Input|ActionEvents|InputActionJump
  (params (Key :type Key%20Structure))
  (:Pressed
    (Utilities|FlowControl|DoOnce false :!label _label
      (:Completed
        (Utilities|FlowControl|ForLoopwithBreak 0 5
          (:LoopBody
            (Physics|AddImpulse (Variables|Default|GetPanela1) (Math|Vector|MakeVector 0.0 0.0 (Variables|Default|Getmultiplicador%20da%20gravidade)) "None" true))
          (:Completed
            (Utilities|FlowControl|Delay 0.5)
            (Utilities|FlowControl|ForLoopwithBreak 0 10
              (:LoopBody
                (Physics|AddImpulse (Variables|Default|GetPanela1) (Math|Vector|MakeVector 0.0 0.0 (* -1.0 (Variables|Default|Getmultiplicador%20da%20gravidade))) "None" true))
              (:Completed
                (Utilities|FlowControl|Delay 0.5)
                (bind _returnvalue (Physics|GetPhysicsLinearVelocity (Variables|Default|GetPanela1) "None"))
                (Physics|AddImpulse (Variables|Default|GetPanela1) (Math|Vector|MakeVector 0.0 0.0 (* -1.0 (.z _returnvalue))) "None" true))))))))
  (:Released
    (goto _label Reset)))

(event Input|AxisEvents|InputAxisMoveForward
  (params (AxisValue :type Float%20%28single-precision%29))
  (Physics|AddImpulse (Variables|Default|GetPanela1) (Math|Vector|MakeVector (* AxisValue (Variables|Default|Getaccelaration%20multiplier)) 0.0 0.0) "None" true))

(event Input|AxisEvents|InputAxisMoveRight
  (params (AxisValue :type Float%20%28single-precision%29))
  (Physics|AddImpulse (Variables|Default|GetPanela1) (Math|Vector|MakeVector 0.0 (* AxisValue (Variables|Default|Getaccelaration%20multiplier)) 0.0) "None" true))

(event Input|AxisEvents|InputAxisMoveForwardArrow
  (params (AxisValue :type Float%20%28single-precision%29))
  (Physics|AddImpulse (Variables|Default|GetPanela2) (Math|Vector|MakeVector (* AxisValue (Variables|Default|Getaccelaration%20multiplier)) 0.0 0.0) "None" true))

(event Input|AxisEvents|InputAxisMoveRightArrow
  (params (AxisValue :type Float%20%28single-precision%29))
  (Physics|AddImpulse (Variables|Default|GetPanela2) (Math|Vector|MakeVector 0.0 (* AxisValue (Variables|Default|Getaccelaration%20multiplier)) 0.0) "None" true))

(fn ConstructionScript)